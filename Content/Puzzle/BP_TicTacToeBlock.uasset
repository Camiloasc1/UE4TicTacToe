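; Clickable board cell for a Tic-Tac-Toe game that shows its owner through a mesh material and an O or X text.
; Clicking or touching sets the owner to O, with no turn or occupancy check in this graph.
; Highlight toggles a preview mark on empty cells only during O's turn, read from the game state.
; OnSetBlockOwner updates material, mark and text visibility to match the owner.
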(event `self.Highlight`
  (params (bOn :type Boolean))
  (bind _ownertext (`self.OwnerText`))
  (bind _astic_tac_toe_game_state (cast `TicTacToeGameState` (`GameplayStatics.GetGameState`)))
  (bind _currentturn (`TicTacToeGameState.CurrentTurn` _astic_tac_toe_game_state))
  (if (and (`|EnumEquality` (`self.BlockOwner`) "EMPTY") (`|EnumEquality` _currentturn "PLAYER_O"))
    (`SceneComponent.SetVisibility` _ownertext bOn false)
    (if bOn
      (`TextRenderComponent.K2_SetText` _ownertext (select `ETicTacToeTurn` _currentturn :`PLAYER_O` "O" :`PLAYER_X` "X" :!type "Text")))))

(event `self.ReceiveActorOnClicked`
  (params (ButtonPressed :type "Key Structure"))
  (set `self.BlockOwner` "PLAYER_O" :!label _label))

(event `self.ReceiveActorOnInputTouchBegin`
  (params (FingerIndex :type "ETouchIndex Enum" :default "Touch1"))
  (goto _label))

(event `self.OnSetBlockOwner`
  (bind _ownertext (`self.OwnerText`))
  (bind _blockowner (`self.BlockOwner`))
  (`PrimitiveComponent.SetMaterial` (`self.BlockMesh`) 0 (select `ETicTacToeBlockOwner` _blockowner :`EMPTY` "/Game/Puzzle/Meshes/BaseMaterial.BaseMaterial" :`PLAYER_O` "/Game/Puzzle/Meshes/BlueMaterial.BlueMaterial" :`PLAYER_X` "/Game/Puzzle/Meshes/OrangeMaterial.OrangeMaterial" :!type "MaterialInterface Object Reference"))
  (`TextRenderComponent.K2_SetText` _ownertext (select `ETicTacToeBlockOwner` _blockowner :`PLAYER_O` "O" :`PLAYER_X` "X" :!type "Text"))
  (`SceneComponent.SetVisibility` _ownertext true false))

(fn `UserConstructionScript`)